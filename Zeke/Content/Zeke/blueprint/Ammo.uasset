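; Ammo projectile actor, apparently a shooting test, that is launched by physics impulse and meant to damage characters.
; On BeginPlay it pushes M9Ammo at the world origin with an impulse scaled from the Gun's location, as the rotated offset is zero.
; AmmoDamage's end overlap calls ApplyDamage with the Police controller as instigator, but no damaged actor is wired.
; Hit is empty, and alternative movement experiments are left disconnected.
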(event OnComponentEndOverlap(AmmoDamage)
  (params (OtherActor :type Actor%20Object%20Reference) (OtherComp :type Primitive%20Component%20Object%20Reference) (OtherBodyIndex :type Integer))
  ;[1 1 1] Does damage to character
  (Game|Damage|ApplyDamage 0 (Math|Conversions|ToFloat(Integer) (Variables|Default|GetAmmoDamagee)) (Pawn|GetController (Variables|Default|GetPolice)) 0))

(event EventBeginPlay
  (bind _gun (Variables|Default|GetGun))
  ;[1 1 1] Testing shooting stuff
  (Physics|AddImpulseatLocation (Variables|Default|GetM9Ammo) (* (+ (Transformation|GetActorLocation _gun) (Math|Vector|RotateVector "0, 0, 0" (Transformation|GetActorRotation _gun))) 5.0) "0, 0, 0" "None"))

(event EventHit
  (params (MyComp :type Primitive%20Component%20Object%20Reference) (Other :type Actor%20Object%20Reference) (OtherComp :type Primitive%20Component%20Object%20Reference) (bSelfMoved :type Boolean) (HitLocation :type Vector :default "0, 0, 0") (HitNormal :type Vector :default "0, 0, 0") (NormalImpulse :type Vector :default "0, 0, 0") (Hit :type Hit%20Result%20Structure%20%28by%20ref%29)))

(fn ConstructionScript)